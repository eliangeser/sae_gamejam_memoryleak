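; Boss enemy actor whose max HP is looked up per wave from an array, with a projectile value derived as a fifth of that HP.
; It registers itself and its camera with GM_GameManager and pushes damage, resets and wave increments to the HUD boss health bar.
; At zero HP in gamemode 2, it plays death animation and sounds, then ends that mode after a delay.
; Face events swap the monitor material for expressions.
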(event Custom|IncrementMaxHp
  (Variables|Default|SetEnemyDead false)
  (bind _output_get (Variables|Default|SetWave%20count (+ (Variables|Default|GetWave%20count) 1)))
  (bind _output_get_2 (Variables|Default|SetCurrentMaxHP (Utilities|Array|Get(acopy) (Variables|Default|GetMaxHPArray) (- _output_get 1))))
  (Variables|Default|SetCurrentHP _output_get_2)
  (CallFunction|SetProjectileValue)
  ;[1 1 1] Health UI Set
  (bind _asgm_game_manager (Utilities|Casting|CastToGM_GameManager (Game|GetGameMode)))
  (Default|UpdateBossHealthBar (Variables|/Game/Project/Elian/GM_GameManager.GM_GameManager_C|GetHUD_Widget _asgm_game_manager) (Variables|Default|GetCurrentHP) (Variables|Default|GetCurrentMaxHP)))

(event Custom|boss_face_angry
  (Rendering|Material|SetMaterialbyName (Variables|Default|GetBossBot) (Utilities|Array|Get(acopy) (Class|PrimitiveComponent|GetMaterialSlotNames (Variables|Default|GetBossBot)) 2) "/Game/Project/Models/BossModel/boss_monitor_mat.boss_monitor_mat"))

(event Custom|boss_face_noface
  (Rendering|Material|SetMaterialbyName (Variables|Default|GetBossBot) (Utilities|Array|Get(acopy) (Class|PrimitiveComponent|GetMaterialSlotNames (Variables|Default|GetBossBot)) 2) "/Game/Project/Models/BossModel/boss_monitor_blank.boss_monitor_blank"))

(event Custom|ResetEnemy
  (Variables|Default|SetWave%20count 1)
  (bind _output_get (Variables|Default|SetCurrentHP (Utilities|Array|Get(acopy) (Variables|Default|GetMaxHPArray))))
  (Variables|Default|SetCurrentMaxHP _output_get)
  (CallFunction|SetProjectileValue)
  ;[1 1 1] Health UI Set
  (bind _asgm_game_manager (Utilities|Casting|CastToGM_GameManager (Game|GetGameMode)))
  (Default|UpdateBossHealthBar (Variables|/Game/Project/Elian/GM_GameManager.GM_GameManager_C|GetHUD_Widget _asgm_game_manager) (Variables|Default|GetCurrentHP) (Variables|Default|GetCurrentMaxHP)))

(event Custom|boss_face_happy
  (Rendering|Material|SetMaterialbyName (Variables|Default|GetBossBot) (Utilities|Array|Get(acopy) (Class|PrimitiveComponent|GetMaterialSlotNames (Variables|Default|GetBossBot)) 2) "/Game/Project/Models/BossModel/boss_monitor_happy1.boss_monitor_happy1"))

(event Custom|SetProjectileValue
  (Variables|Default|SetprojectileValue (/ (Variables|Default|GetCurrentMaxHP) 5)))

(event Custom|boss_face_sleepy
  (Rendering|Material|SetMaterialbyName (Variables|Default|GetBossBot) (Utilities|Array|Get(acopy) (Class|PrimitiveComponent|GetMaterialSlotNames (Variables|Default|GetBossBot)) 2) "/Game/Project/Models/BossModel/boss_monitor_sleepy.boss_monitor_sleepy"))

(event EventBeginPlay
  (bind _output_get (Variables|Default|SetCurrentMaxHP (Utilities|Array|Get(acopy) (Variables|Default|GetMaxHPArray))))
  (Variables|Default|SetCurrentHP _output_get)
  (CallFunction|SetProjectileValue)
  (bind _asgm_game_manager (Utilities|Casting|CastToGM_GameManager (Game|GetGameMode)))
  (Variables|Default|SetGameManager _asgm_game_manager)
  (Variables|/Game/Project/Elian/GM_GameManager.GM_GameManager_C|SetEnemy _asgm_game_manager self)
  (CallFunction|BossFaceSleepy)
  (Variables|/Game/Project/Elian/GM_GameManager.GM_GameManager_C|SetCameraEnemy (Variables|Default|GetGameManager) (Variables|Default|GetCamera))
  (bind _asgi_upgrade_manager (Utilities|Casting|CastToGI_UpgradeManager (Game|GetGameInstance)))
  (Variables|Default|SetGameInstance _asgi_upgrade_manager))

(event Game|Damage|EventAnyDamage
  (params (Damage :type Float%20%28single-precision%29) (DamageType :type Damage%20Type%20Object%20Reference) (InstigatedBy :type Controller%20Object%20Reference) (DamageCauser :type Actor%20Object%20Reference))
  (bind _output_get (Variables|Default|SetCurrentHP (Math|Integer|Clamp(Integer) (Math|Float|Truncate (- (Variables|Default|GetCurrentHP) Damage)) 0 (Variables|Default|GetCurrentMaxHP))))
  (bind _asgm_game_manager (Utilities|Casting|CastToGM_GameManager (Game|GetGameMode)))
  (Default|UpdateBossHealthBar (Variables|/Game/Project/Elian/GM_GameManager.GM_GameManager_C|GetHUD_Widget _asgm_game_manager) (Variables|Default|GetCurrentHP) (Variables|Default|GetCurrentMaxHP))
  (if (<= _output_get 0)
    (if (== (Variables|/Game/Project/Elian/GM_GameManager.GM_GameManager_C|GetGamemodeInteger (Variables|Default|GetGameManager)) 2)
      (if (not (Variables|Default|GetEnemyDead))
        (Variables|Default|SetEnemyDead true)
        (Components|Animation|PlayAnimation (Variables|Default|GetBossBot) "/Game/Project/Mete/Enemy/Models/newModels/boss_death.boss_death" false)
        (bind _asgi_upgrade_manager (Utilities|Casting|CastToGI_UpgradeManager (Game|GetGameInstance)))
        (Default|PlayEnemySFX _asgi_upgrade_manager "DeathSound1")
        (Default|PlayEnemySFX _asgi_upgrade_manager "DeathSound2")
        (Default|PlayEnemySFX _asgi_upgrade_manager "DeathSound3")
        (Utilities|FlowControl|Delay 1.0)
        (Default|EndGamemode2 (Variables|Default|GetGameManager))))))

(fn ConstructionScript)