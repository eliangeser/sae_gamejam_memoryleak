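; Projectile that displays an integer as 3D digit meshes and deals it as damage to the player or enemies.
; Colliding number projectiles destroy the smaller one, or both when equal; hits spawn Niagara effects and destroy it once bounced.
; SetNumber builds value-tinted digits, while BeginPlay sets speed by enemy wave.
; When the player is Overflowed, digits turn green, re-randomise, and hits deal enemies' max HP.
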(event OnProjectileBounce(ProjectileMovement)
  (params (ImpactResult :type Hit%20Result%20Structure%20%28by%20ref%29) (ImpactVelocity :type Vector%20%28by%20ref%29 :default "0, 0, 0"))
  (bind _output_get (Variables|Default|SethasBounced true)))

(event Custom|Matrix%20Number
  (params (NumberInput :type Integer))
  (Components|DestroyComponent (Variables|Default|GetMeshArray))
  (CallFunction|SetNumber NumberInput))

(event Custom|PlayHitSFX
  (bind _asgi_upgrade_manager (Utilities|Casting|CastToGI_UpgradeManager (Game|GetGameInstance)))
  (Default|PlayProjectileSFX _asgi_upgrade_manager "KillNumber" 0.0))

(event Custom|PlayWallCollideSFX
  ;[1 1 1] Not in use ATM
  (bind _asgi_upgrade_manager (Utilities|Casting|CastToGI_UpgradeManager (Game|GetGameInstance)))
  (Default|PlayProjectileSFX _asgi_upgrade_manager "CollideWall" 0.0))

(event Custom|SetNumber
  (params (NumberInput :type Integer))
  (bind _output_get (Variables|Default|SetNumberInt NumberInput))
  (for _index (range 0 (- (Utilities|String|Len (Utilities|String|ToString(Integer) _output_get)) 1))
    (bind _returnvalue (Game|AddComponentbyClass "/Script/Engine.StaticMeshComponent" false))
    (bind _output_get_2 (Variables|Default|SetAddedNumberMesh _returnvalue))
    (Utilities|Array|Add (Variables|Default|GetMeshArray) _output_get_2)
    (if (Variables|Default|GetOverflowed)
      (Rendering|Material|SetMaterial _output_get_2 0 "/Game/Project/Mete/Materials/Green.Green")
      (else
        (bind _returnvalue_2 (Rendering|Material|CreateDynamicMaterialInstance "/Game/Project/Mete/Materials/Blue.Blue" "None" "None" :!class /Script/Engine.KismetMaterialLibrary))
        (Rendering|Material|SetMaterial _output_get_2 0 _returnvalue_2)
        (Rendering|Material|SetScalarParameterValue _returnvalue_2 "NumberVal" (Math|Float|Clamp(Float) (/ (Math|Conversions|ToFloat(Integer) (Math|Integer|Clamp(Integer) (Variables|Default|GetNumberInt) 1 999)) 999.0)) :!class /Script/Engine.MaterialInstanceDynamic)))
    (CallFunction|MeshMaterialConstructor (Math|Conversions|ToInteger(Byte) (Utilities|Array|Get(acopy) (Utilities|String|GetCharacterArrayfromString (Utilities|String|ToString(Integer) _output_get)) _index)) _returnvalue)
    (Transformation|SetWorldScale3D _returnvalue "2.000000,2.000000,2.000000")
    (Transformation|SetRelativeLocation _returnvalue (Math|Vector|MakeVector (* (- (Math|Conversions|ToFloat(Integer) _index) (Math|Conversions|ToFloat(Integer) (/ (- (Utilities|Array|Length (Utilities|String|GetCharacterArrayfromString (Utilities|String|ToString(Integer) _output_get))) 1) 2))) 5e+01) 0.0 0.0) false false)
    (Collision|SetCollisionEnabled _returnvalue "NoCollision")
    (Collision|SetCollisionResponsetoAllChannels _returnvalue "ECR_Ignore"))
  (Transformation|SetWorldRotation (Variables|Default|GetBox) "0.000000,90.000000,0.000000" false false))

(event Collision|EventActorBeginOverlap
  (params (OtherActor :type Actor%20Object%20Reference))
  (bind _numberint (Variables|Default|GetNumberInt))
  ;[1 1 1] Hit Player
  (bind _asbp_top_down_character (Utilities|Casting|CastToBP_TopDownCharacter OtherActor)
    (:then
      (Game|Damage|ApplyDamage _asbp_top_down_character (Math|Conversions|ToFloat(Integer) (Variables|Default|GetNumberInt)) 0 0)
      (CallFunction|PlayHitSFX)
      (Actor|DestroyActor))
    (:CastFailed
      ;[1 1 1] Hit Enemy
      (bind _asenemy (Utilities|Casting|CastToEnemy OtherActor)
        (:then
          (if (Variables|Default|GetOverflowed)
            (Game|Damage|ApplyDamage _asenemy (Math|Conversions|ToFloat(Integer) (Variables|/Game/Project/Mete/Enemy/Blueprints/Enemy.Enemy_C|GetCurrentMaxHP _asenemy)) 0 0)
            (else
              (Game|Damage|ApplyDamage _asenemy (Math|Conversions|ToFloat(Integer) (Variables|Default|GetNumberInt)) 0 0)))
          (CallFunction|PlayHitSFX)
          (Actor|DestroyActor))
        (:CastFailed
          (bind _asbp_number_projectile (Utilities|Casting|CastToBP_NumberProjectile OtherActor))
          (CallFunction|PlayHitSFX)
          (if (== (Variables|BP_NumberProjectile_C|GetNumberInt _asbp_number_projectile) _numberint)
            (Actor|DestroyActor _asbp_number_projectile)
            (Actor|DestroyActor)
            (elif (> (Variables|BP_NumberProjectile_C|GetNumberInt _asbp_number_projectile) _numberint)
              (Actor|DestroyActor)
              (else
                (Actor|DestroyActor _asbp_number_projectile)))))))))

(event EventTick
  (params (DeltaSeconds :type Float%20%28single-precision%29))
  (Components|Box|SetBoxExtent (Variables|Default|GetBox) (Math|Vector|MakeVector (Math|Interpolation|FInterpTo 0.1 (Math|Conversions|ToFloat(Integer) (* (Utilities|Array|Length (Utilities|String|GetCharacterArrayfromString (Utilities|String|ToString(Integer) (stale Custom|SetNumber _output_get)))) 30)) DeltaSeconds 0.001) 3e+01 32.0) true)
  (bind _newtrack_0 (Timeline|Timeline Play)
    (:Update
      (Transformation|SetWorldScale3D (Variables|Default|GetBox) (Math|Vector|MakeVector _newtrack_0 _newtrack_0 _newtrack_0))
      (if (Variables|Default|GetOverflowed)
        (Utilities|FlowControl|Delay 0.5)
        (CallFunction|MatrixNumber (Math|Random|RandomIntegerinRange 1 2147483647))))))

(event Collision|EventHit
  (params (MyComp :type Primitive%20Component%20Object%20Reference) (Other :type Actor%20Object%20Reference) (OtherComp :type Primitive%20Component%20Object%20Reference) (bSelfMoved :type Boolean) (HitLocation :type Vector :default "0, 0, 0") (HitNormal :type Vector :default "0, 0, 0") (NormalImpulse :type Vector :default "0, 0, 0") (Hit :type Hit%20Result%20Structure%20%28by%20ref%29))
  (AddComponent|AddNiagaraComponent false)
  (if (stale OnProjectileBounce(ProjectileMovement) _output_get)
    (Actor|DestroyActor)))

(event EventBeginPlay
  (bind _projectilemovement (Variables|Default|GetProjectileMovement))
  (bind _returnvalue (Actor|GetActorOfClass "/Game/Project/Petru/Player/Character/BP_TopDownCharacter.BP_TopDownCharacter_C"))
  (bind _output_get (Variables|Default|SetOverflowed (Variables|/Game/Project/Petru/Player/Character/BP_TopDownCharacter.BP_TopDownCharacter_C|GetbOverflowed _returnvalue)))
  (if _output_get
    (CallFunction|MatrixNumber (Math|Random|RandomIntegerinRange 1 2147483647))
    (else
      (bind _returnvalue_2 (Actor|GetActorOfClass "/Game/Project/Mete/Enemy/Blueprints/Enemy.Enemy_C"))
      (switch int (Variables|/Game/Project/Mete/Enemy/Blueprints/Enemy.Enemy_C|GetWave%20count _returnvalue_2)
        (:1
          (Variables|/Script/Engine.ProjectileMovementComponent|SetInitialSpeed _projectilemovement 2.5e+03))
        (:3
          (Variables|/Script/Engine.ProjectileMovementComponent|SetInitialSpeed _projectilemovement 3e+03))
        (:5
          (Variables|/Script/Engine.ProjectileMovementComponent|SetInitialSpeed _projectilemovement 3.5e+03))
        (:7
          (Variables|/Script/Engine.ProjectileMovementComponent|SetInitialSpeed _projectilemovement 4e+03))
        (:9
          (Variables|/Script/Engine.ProjectileMovementComponent|SetInitialSpeed _projectilemovement 5e+03))
        (:10
          (Variables|/Script/Engine.ProjectileMovementComponent|SetInitialSpeed _projectilemovement 6e+03))))))

(fn ConstructionScript
  (Variables|/Script/Engine.MovementComponent|SetVelocity (Variables|Default|GetProjectileMovement) (Variables|Default|GetNumber%20Rotation)))

(fn MeshMaterialConstructor
  (params (Value :type Integer) (Mesh%20Ref :type Static%20Mesh%20Component%20Object%20Reference))
  (if (== Value 1)
    (Components|StaticMesh|SetStaticMesh Mesh%20Ref "/Game/Project/Mete/Enemy/Models/Numbers/numbers_n_1.numbers_n_1")
    (elif (== Value 2)
      (Components|StaticMesh|SetStaticMesh Mesh%20Ref "/Game/Project/Mete/Enemy/Models/Numbers/numbers_n_2.numbers_n_2")
      (elif (== Value 3)
        (Components|StaticMesh|SetStaticMesh Mesh%20Ref "/Game/Project/Mete/Enemy/Models/Numbers/numbers_n_3.numbers_n_3")
        (elif (== Value 4)
          (Components|StaticMesh|SetStaticMesh Mesh%20Ref "/Game/Project/Mete/Enemy/Models/Numbers/numbers_n_4.numbers_n_4")
          (elif (== Value 5)
            (Components|StaticMesh|SetStaticMesh Mesh%20Ref "/Game/Project/Mete/Enemy/Models/Numbers/numbers_n_5.numbers_n_5")
            (elif (== Value 6)
              (Components|StaticMesh|SetStaticMesh Mesh%20Ref "/Game/Project/Mete/Enemy/Models/Numbers/numbers_n_6.numbers_n_6")
              (elif (== Value 7)
                (Components|StaticMesh|SetStaticMesh Mesh%20Ref "/Game/Project/Mete/Enemy/Models/Numbers/numbers_n_7.numbers_n_7")
                (elif (== Value 8)
                  (Components|StaticMesh|SetStaticMesh Mesh%20Ref "/Game/Project/Mete/Enemy/Models/Numbers/numbers_n_8.numbers_n_8")
                  (elif (== Value 9)
                    (Components|StaticMesh|SetStaticMesh Mesh%20Ref "/Game/Project/Mete/Enemy/Models/Numbers/numbers_n_9.numbers_n_9")
                    (elif (== Value 0)
                      (Components|StaticMesh|SetStaticMesh Mesh%20Ref "/Game/Project/Mete/Enemy/Models/Numbers/numbers_n_0.numbers_n_0"))))))))))))