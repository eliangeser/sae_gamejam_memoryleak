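; Collectable number actor that spawns as a random digit from 1 to 6 and moves via a ProjectileMovement component.
; On BeginPlay it gets its value from the GM_GameManager NumberProvider, then an if-chain sets the matching mesh and color material and applies a fixed rotation.
; The Construction Script sets the projectile velocity from the NumberRotation variable, and BeginPlay activates the movement.
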(event EventBeginPlay
  (bind _numbers (Variables|Default|GetNumbers))
  ;[1 1 1] Get Random Number with Probability
  (bind _asgm_game_manager (Utilities|Casting|CastToGM_GameManager (Game|GetGameMode)))
  (bind _outputnumber (Default|GetRandomNumber (Variables|/Game/Project/Elian/GM_GameManager.GM_GameManager_C|GetNumberProvider _asgm_game_manager)))
  (Components|Activation|SetActive (Variables|Default|GetProjectileMovement) true false)
  (bind _output_get (Variables|Default|SetNumberValueInt _outputnumber))
  (bind _output_get_2 (Variables|Default|SetNumberValueInt _outputnumber))
  (bind _output_get_3 (Variables|Default|SetNumberValueInt _outputnumber))
  (bind _output_get_4 (Variables|Default|SetNumberValueInt _outputnumber))
  (bind _output_get_5 (Variables|Default|SetNumberValueInt _outputnumber))
  (bind _output_get_6 (Variables|Default|SetNumberValueInt _outputnumber))
  (if (== _output_get 1)
    (Components|StaticMesh|SetStaticMesh _numbers "/Game/Project/Mete/Enemy/Models/Numbers/numbers_n_1.numbers_n_1")
    (Rendering|Material|SetMaterial _numbers 0 "/Game/Project/Mete/Materials/Blue.Blue")
    (Transformation|SetActorRotation "0.000000,90.000000,0.000000" :!label _label)
    (elif (== _output_get_2 2)
      (Components|StaticMesh|SetStaticMesh _numbers "/Game/Project/Mete/Enemy/Models/Numbers/numbers_n_2.numbers_n_2")
      (Rendering|Material|SetMaterial _numbers 0 "/Game/Project/Mete/Materials/Green.Green")
      (goto _label)
      (elif (== _output_get_3 3)
        (Components|StaticMesh|SetStaticMesh _numbers "/Game/Project/Mete/Enemy/Models/Numbers/numbers_n_3.numbers_n_3")
        (Rendering|Material|SetMaterial _numbers 0 "/Game/Project/Mete/Materials/Pink.Pink")
        (goto _label)
        (elif (== _output_get_4 4)
          (Components|StaticMesh|SetStaticMesh _numbers "/Game/Project/Mete/Enemy/Models/Numbers/numbers_n_4.numbers_n_4")
          (Rendering|Material|SetMaterial _numbers 0 "/Game/Project/Mete/Materials/Red.Red")
          (goto _label)
          (elif (== _output_get_5 5)
            (Components|StaticMesh|SetStaticMesh _numbers "/Game/Project/Mete/Enemy/Models/Numbers/numbers_n_5.numbers_n_5")
            (Rendering|Material|SetMaterial _numbers 0 "/Game/Project/Mete/Materials/Yellow.Yellow")
            (goto _label)
            (elif (== _output_get_6 6)
              (Components|StaticMesh|SetStaticMesh _numbers "/Game/Project/Mete/Enemy/Models/Numbers/numbers_n_6.numbers_n_6")
              (Rendering|Material|SetMaterial _numbers 0 "/Game/Project/Mete/Materials/Purple.Purple")
              (goto _label))))))))

(fn ConstructionScript
  (Variables|/Script/Engine.MovementComponent|SetVelocity (Variables|Default|GetProjectileMovement) (Variables|Default|GetNumber%20Rotation)))