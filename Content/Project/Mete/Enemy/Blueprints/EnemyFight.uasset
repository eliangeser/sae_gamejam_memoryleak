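; EnemyFight is an enemy actor that turns on its yaw while firing collectable number actors.
; BeginPlay enables physics on its mesh, and Tick plays a timeline that drives the actor's yaw.
; Timeline updates spawn BP_CollectableNumber at the spawn arrow, passing its forward vector, with a cooldown flag and random delay spacing the shots.
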(event EventBeginPlay
  (Physics|SetSimulatePhysics (Variables|Character|GetMesh) true))

(event Collision|EventActorBeginOverlap
  (params (OtherActor :type Actor%20Object%20Reference)))

(event EventTick
  (params (DeltaSeconds :type Float%20%28single-precision%29))
  (bind _projectilespawnarrow (Variables|Default|GetProjectileSpawnArrow))
  (bind _newtrack_0 (Timeline|Enemy%20Rotate%20Timeline Play)
    (:Update
      (Transformation|SetActorRotation (Math|Rotator|MakeRotator 0.0 0.0 (.z _newtrack_0)))
      (if (not (Variables|Default|GetShoot%20on%20CD))
        (Variables|Default|SetShoot%20on%20CD true)
        (Game|SpawnActorfromClass "/Game/Enemy/Blueprints/BP_CollectableNumber.BP_CollectableNumber_C" (Transformation|GetWorldTransform _projectilespawnarrow) "AlwaysSpawn" "MultiplyWithRoot" 0 (Math|Rotator|GetRotationXVector (Transformation|GetSocketRotation _projectilespawnarrow "None")) 0)
        (Utilities|FlowControl|Delay (Math|Random|RandomFloatinRange 0.33 3.0))
        (Variables|Default|SetShoot%20on%20CD false)))))

(fn ConstructionScript)