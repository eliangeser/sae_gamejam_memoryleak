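; BP_Camera is a camera actor that tracks the point between the top-down player character and an enemy.
; On BeginPlay it finds one actor of each class, then every Tick moves its root to their midpoint in X and Y.
; MoveCameraToEnemy and MoveCameraToPlayer blend the player controller's view target to the enemy or back to this camera, rather than to the character itself.
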(event Custom|MoveCameraToEnemy
  (Game|Player|SetViewTargetwithBlend (Game|GetPlayerController 0) (stale EventBeginPlay _returnvalue) 1.0 "VTBlend_Linear" 0.0 false))

(event Custom|MoveCameraToPlayer
  (Game|Player|SetViewTargetwithBlend (Game|GetPlayerController 0) self 1.0 "VTBlend_Linear" 0.0 false))

(event EventBeginPlay
  (bind _returnvalue (Actor|GetActorOfClass "/Game/Project/Mete/Enemy/Blueprints/Enemy.Enemy_C"))
  (bind _returnvalue_2 (Actor|GetActorOfClass "/Game/Project/Petru/Player/Character/BP_TopDownCharacter.BP_TopDownCharacter_C")))

(event Collision|EventActorBeginOverlap
  (params (OtherActor :type Actor%20Object%20Reference)))

(event EventTick
  (params (DeltaSeconds :type Float%20%28single-precision%29))
  (Transformation|SetWorldLocation (Variables|Default|GetDefaultSceneRoot) (Math|Vector|MakeVector (.x (/ (+ (Transformation|GetActorLocation (stale EventBeginPlay _returnvalue_2)) (Transformation|GetActorLocation (stale EventBeginPlay _returnvalue))) 2)) (.y (/ (+ (Transformation|GetActorLocation (stale EventBeginPlay _returnvalue_2)) (Transformation|GetActorLocation (stale EventBeginPlay _returnvalue))) 2)) 0.0) false false))

(fn ConstructionScript)