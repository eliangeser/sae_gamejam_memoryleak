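; Game manager (by its name, the game mode) that runs the loop: main menu, timed number-collecting phase, boss fight, then shop between waves.
; It creates the UI widgets, number provider and text converter; a Tick countdown switches collecting to fighting.
; Phase, pause and resume events drive the boss's look, camera and music via the GameInstance upgrade manager.
; It also owns the number-ammo magazine, with recursive removal spilling across entries.
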(event Custom|DoubleChanceOfNumber
  (params (InputNumber :type Integer))
  ;[1 1 1] Spawning Numbers in Collect Phase (move to Enemy?)
  (Default|DoubleChanceOfNumber (Variables|Default|GetNumberProvider) InputNumber))

(event Custom|EnterGamemode1
  (bind _enemy (Variables|Default|GetEnemy))
  ;[1 1 1] Managing Game States
  (Default|SwitchBossMeshtoNormal (Variables|Default|GetEnemy))
  (bind _asbp_top_down_character (Utilities|Casting|CastToBP_TopDownCharacter (Game|GetPlayerCharacter 0)))
  (bind _returnvalue (Actor|GetActorOfClass "/Game/Project/Mete/Camera/Blueprints/BP_Camera.BP_Camera_C"))
  (Default|MoveCameratoPlayer _returnvalue)
  (Default|EnableMovement _asbp_top_down_character)
  (Default|BossFaceSleepy (Variables|Default|GetEnemy))
  (Default|FadeOutMenuMusic (Variables|Default|GetUpgradeManager))
  (Default|FadeOutShopMusic (Variables|Default|GetUpgradeManager))
  (if (Variables|Default|GetbCollectSFXStarted)
    (Default|SetCollectMusicVolume (Variables|Default|GetUpgradeManager) 1.0)
    (else
      (Default|StartCollectMusic (Variables|Default|GetUpgradeManager))
      (Variables|Default|SetbCollectSFXStarted true)))
  (Variables|Default|SetGamemodeInteger 1)
  (CallFunction|ResetCountdown)
  (Default|UpdateBossHealthBar (Variables|Default|GetHUD_Widget) (Variables|/Game/Project/Mete/Enemy/Blueprints/Enemy.Enemy_C|GetCurrentHP _enemy) (Variables|/Game/Project/Mete/Enemy/Blueprints/Enemy.Enemy_C|GetCurrentMaxHP _enemy))
  (CallFunction|ShowHUD)
  (CallFunction|TransformHUDtoCollect))

(event Custom|StartCountdown
  ;[1 1 1] CountDown
  (Variables|Default|SetbRunTimer true))

(event Custom|DebugMagazineLength
  ;[1 1 1] Magazine
  (Development|PrintString (Utilities|String|ToString(Integer) (Utilities|Array|Length (Variables|Default|GetMagazine)))))

(event Custom|RemoveAmmoAmount
  (params (AmountToRemove :type Integer))
  (bind _magazine (Variables|Default|GetMagazine))
  (bind _output (Utilities|Array|Get(acopy) _magazine))
  ;[1 1 1] Magazine
  (if (> AmountToRemove 0)
    (bind _output_get (Variables|Default|SetAmmoLossCount AmountToRemove))
    (if (> _output_get _output)
      (bind _output_get_2 (Variables|Default|SetAmmoLossCount (- (Variables|Default|GetAmmoLossCount) (Utilities|Array|Get(acopy) (Variables|Default|GetMagazine)))))
      (CallFunction|RemoveTopAmmo)
      (if (> (Utilities|Array|Length (Variables|Default|GetMagazine)) 0)
        (CallFunction|RemoveAmmoAmount _output_get_2))
      (elif (> (- _output (Variables|Default|GetAmmoLossCount)) 0)
        (Utilities|Array|SetArrayElem (Variables|Default|GetMagazine) 0 (- _output (Variables|Default|GetAmmoLossCount)))
        (CallFunction|UpdateMagazineUI)
        (else
          (CallFunction|RemoveTopAmmo))))))

(event Custom|RemoveTopAmmo
  ;[1 1 1] Magazine
  (Utilities|Array|RemoveIndex (Variables|Default|GetMagazine))
  (CallFunction|UpdateMagazineUI))

(event Custom|OpenPauseMenu
  (bind _gamemodeinteger (Variables|Default|GetGamemodeInteger))
  (bind _upgrademanager (Variables|Default|GetUpgradeManager))
  (bind _returnvalue (== _gamemodeinteger 1))
  ;[1 1 1] UI Logic
  (Default|SwitchBossMeshtoStatic (Variables|Default|GetEnemy))
  (bind _returnvalue_2 (Actor|GetActorOfClass "/Game/Project/Mete/Camera/Blueprints/BP_Camera.BP_Camera_C"))
  (Default|MoveCameratoEnemy _returnvalue_2)
  (Default|BossFaceNoface (Variables|Default|GetEnemy))
  (if (== (Variables|Default|GetGamemodeInteger) 2)
    (Default|SetFigthLoopVolume _upgrademanager 0.0)
    (Default|SetFightLoopPausedVolume _upgrademanager 1.0)
    (else
      (Development|PrintString (Utilities|String|ToString(Boolean) _returnvalue))
      (if _returnvalue
        (Default|SetCollectMusicVolume (Variables|Default|GetUpgradeManager) 0.65))))
  (CallFunction|StopCountdown)
  (Game|SetGamePaused true)
  (Utilities|FlowControl|Delay 1.0)
  (Default|PlayMenuSFX (Variables|Default|GetUpgradeManager) "OpenPause")
  (bind _returnvalue_3 (UserInterface|CreateWidget "/Game/Project/Elian/GUI/WB_PauseMenu.WB_PauseMenu_C"))
  (UserInterface|Viewport|AddtoViewport _returnvalue_3 0)
  (Variables|/Script/Engine.PlayerController|SetbShowMouseCursor (Game|GetPlayerController 0) true))

(event Custom|UpdateMagazineUI
  ;[1 1 1] Magazine
  (Default|UpdateMagazineUI (Variables|Default|GetHUD_Widget)))

(event Custom|StopCountdown
  ;[1 1 1] CountDown
  (Variables|Default|SetbRunTimer false))

(event Custom|DoubleChanceOddNumbers
  ;[1 1 1] Spawning Numbers in Collect Phase (move to Enemy?)
  (Default|DoubleChanceOfOddNumbers (Variables|Default|GetNumberProvider)))

(event Custom|ExitShop
  (bind _enemy (Variables|Default|GetEnemy))
  ;[1 1 1] Managing Game States
  (Default|IncrementMaxHp (Variables|Default|GetEnemy))
  (Default|UpdateBossHealthBar (Variables|Default|GetHUD_Widget) (Variables|/Game/Project/Mete/Enemy/Blueprints/Enemy.Enemy_C|GetCurrentHP _enemy) (Variables|/Game/Project/Mete/Enemy/Blueprints/Enemy.Enemy_C|GetCurrentMaxHP _enemy))
  ;;[1 1 1] Only Add them after round 5
  (if (== (Variables|Default|GetWaveCount) 5)
    (Default|AddChancesUpgrades (Variables|Default|GetUpgradeManager)))
  (CallFunction|EnterGamemode1))

(event Custom|ResetCountdown
  ;[1 1 1] CountDown
  (Variables|Default|SetCurrentTimer 0.0)
  (bind _output_get (Variables|Default|SetCurrentCountdownValue (Variables|Default|GetMaxCountdownValue)))
  (Default|UpdateTimer (Variables|Default|GetHUD_Widget) _output_get))

(event Custom|EnterGamemode2
  ;[1 1 1] Managing Game States
  (CallFunction|TransformHUDtoFight)
  (bind _outactors (Actor|GetAllActorsOfClass "/Game/Project/Mete/Enemy/Blueprints/BP_CollectableNumber.BP_CollectableNumber_C"))
  (for _array_element _outactors
    (Actor|DestroyActor _array_element))
  (Default|BossFaceAngry (Variables|Default|GetEnemy))
  (Default|SetCollectMusicVolume (Variables|Default|GetUpgradeManager) 0.0)
  (if (Variables|/Game/Project/Elian/SoundManager/SFXManager.SFXManager_C|GetbFightLoopSetup (Variables|/Game/Project/Elian/GI_UpgradeManager.GI_UpgradeManager_C|GetSFXManager (Variables|Default|GetUpgradeManager)))
    _
    (else
      (Default|StartFightMusic (Variables|Default|GetUpgradeManager))))
  (Variables|Default|SetGamemodeInteger 2)
  ;;[1 1 1] Still need this?
  (bind _asbp_top_down_character (Utilities|Casting|CastToBP_TopDownCharacter (Game|Player|GetPlayerPawn 0)))
  (Variables|/Game/Project/Petru/Player/Character/BP_TopDownCharacter.BP_TopDownCharacter_C|SetbSecondPhase _asbp_top_down_character true)
  (Variables|/Script/Engine.PlayerController|SetbShowMouseCursor (Game|GetPlayerController 0) true))

(event Custom|DoubleChanceEvenNumbers
  ;[1 1 1] Spawning Numbers in Collect Phase (move to Enemy?)
  (Default|DoubleChanceOfEvenNumbers (Variables|Default|GetNumberProvider)))

(event Custom|InitSettingsUI
  ;[1 1 1] UI Logic
  (bind _returnvalue (UserInterface|CreateWidget "/Game/Project/Mete/TransferForlder/WB_SettingsMenu.WB_SettingsMenu_C"))
  (Variables|Default|SetSettingsMenu _returnvalue))

(event Custom|ShowSettings
  (params (bIsMainMenuSettings :type Boolean))
  (bind _settingsmenu (Variables|Default|GetSettingsMenu))
  ;[1 1 1] UI Logic
  (UserInterface|Viewport|AddtoViewport _settingsmenu 0)
  (Variables|/Game/Project/Mete/TransferForlder/WB_SettingsMenu.WB_SettingsMenu_C|SetbMainMenuSettings _settingsmenu bIsMainMenuSettings))

(event Custom|InitMainMenu
  ;[1 1 1] UI Logic
  (bind _returnvalue (UserInterface|CreateWidget "/Game/Project/Elian/GUI/WB_MainMenu.WB_MainMenu_C"))
  (Variables|Default|SetWB_MainMenu _returnvalue))

(event Custom|EnterShopMode
  (bind _outactors (Actor|GetAllActorsOfClass "/Game/Project/Mete/Enemy/Blueprints/BP_NumberProjectile.BP_NumberProjectile_C"))
  ;[1 1 1] Managing Game States
  (Actor|DestroyActor _outactors)
  (Variables|Default|SetWaveCount (+ (Variables|Default|GetWaveCount) 1))
  (Default|FadeinShopMusic (Variables|Default|GetUpgradeManager))
  (CallFunction|HideHUD)
  (CallFunction|ClearMagazine)
  (Default|ResetMagazineTotalValue (Variables|Default|GetHUD_Widget))
  (CallFunction|ShowShop)
  (Variables|Default|SetGamemodeInteger 0))

(event Custom|EndGamemode2
  ;[1 1 1] Managing Game States
  (CallFunction|HideHUD)
  (CallFunction|EnterShopMode)
  (Default|TurnFightLoopOff (Variables|Default|GetUpgradeManager)))

(event Custom|ClearMagazine
  ;[1 1 1] Magazine
  (Utilities|Array|Clear (Variables|Default|GetMagazine))
  (Default|UpdateMagazineUI (Variables|Default|GetHUD_Widget)))

(event Custom|DebugReduceTimerTo3Seconds
  ;[1 1 1] DEBUG
  (Variables|Default|SetCurrentCountdownValue 3))

(event Custom|DEBUG_Event%28M%29
  ;[1 1 1] DEBUG
)

(event Custom|TransformHUDToFight
  ;[1 1 1] UI Logic
  (Default|TransformtoFight (Variables|Default|GetHUD_Widget)))

(event Custom|ShowMainMenu
  ;[1 1 1] UI Logic
  (UserInterface|Viewport|AddtoViewport (Variables|Default|GetWB_MainMenu) 0)
  (Default|FadeinMenuMusic (Variables|Default|GetUpgradeManager)))

(event Custom|TransformHUDToCollect
  ;[1 1 1] UI Logic
  (Default|TransformtoCollect (Variables|Default|GetHUD_Widget)))

(event Custom|ResumeGame
  (bind _upgrademanager (Variables|Default|GetUpgradeManager))
  ;[1 1 1] Managing Game States
  (Default|SwitchBossMeshtoNormal (Variables|Default|GetEnemy))
  (bind _returnvalue (Actor|GetActorOfClass "/Game/Project/Mete/Camera/Blueprints/BP_Camera.BP_Camera_C"))
  (Default|MoveCameratoPlayer _returnvalue)
  (if (== (Variables|Default|GetGamemodeInteger) 2)
    (Default|BossFaceAngry (Variables|Default|GetEnemy))
    (Default|SetFigthLoopVolume _upgrademanager 1.0)
    (Default|SetFightLoopPausedVolume _upgrademanager 0.0)
    (Utilities|FlowControl|Delay 1.0 :!label _label)
    (Game|SetGamePaused false)
    (CallFunction|StartCountdown)
    (elif (== (Variables|Default|GetGamemodeInteger) 1)
      (Default|BossFaceSleepy (Variables|Default|GetEnemy))
      (Default|SetCollectMusicVolume (Variables|Default|GetUpgradeManager) 1.0)
      (goto _label))))

(event Custom|EndGame
  ;[1 1 1] Managing Game States
  (Default|ClearCurrentUpgrades (Variables|Default|GetUpgradeManager))
  (Default|RemoveChancesUpgrades (Variables|Default|GetUpgradeManager))
  (bind _returnvalue (Game|GetCurrentLevelName true))
  (Game|OpenLevel(byName) (Utilities|String|StringToName _returnvalue)))

(event Custom|InitHUD
  ;[1 1 1] UI Logic
  (bind _returnvalue (UserInterface|CreateWidget "/Game/Project/Elian/GUI/WB_HUD.WB_HUD_C"))
  (Variables|Default|SetHUD_Widget _returnvalue)
  (CallFunction|ResetCountdown))

(event Custom|ShowShop
  ;[1 1 1] UI Logic
  (UserInterface|Viewport|AddtoViewport (Variables|Default|GetWB_Shop) 0)
  (Variables|/Script/Engine.PlayerController|SetbShowMouseCursor (Game|GetPlayerController 0) true)
  (Default|OpenShop (Variables|Default|GetWB_Shop)))

(event Custom|HideHUD
  ;[1 1 1] UI Logic
  (Widget|RemovefromParent (Variables|Default|GetHUD_Widget)))

(event Custom|ShowHUD
  ;[1 1 1] UI Logic
  (UserInterface|Viewport|AddtoViewport (Variables|Default|GetHUD_Widget) 0)
  (CallFunction|ResetCountdown)
  (CallFunction|StartCountdown))

(event Custom|AddAmmo
  (params (NewNumber :type Integer))
  ;[1 1 1] Magazine
  (if (> NewNumber 0)
    (CallFunction|DebugMagazineLength)
    (Utilities|Array|Insert (Variables|Default|GetMagazine) NewNumber)
    (CallFunction|DebugMagazineLength)
    (Default|UpdateMagazineUI (Variables|Default|GetHUD_Widget))))

(event Custom|InitShop
  ;[1 1 1] UI Logic
  (bind _returnvalue (UserInterface|CreateWidget "/Game/Project/Elian/GUI/WB_Shop.WB_Shop_C"))
  (Variables|Default|SetWB_Shop _returnvalue))

(event EventBeginPlay
  (bind _asgi_upgrade_manager (Utilities|Casting|CastToGI_UpgradeManager (Game|GetGameInstance)))
  (Variables|Default|SetUpgradeManager _asgi_upgrade_manager)
  ;[1 1 1] Setup RandomNumberProvider (Move to Enemy?)
  (bind _returnvalue (Game|ConstructObjectfromClass "/Game/Project/Elian/NumberProvider/NumberProvider.NumberProvider_C"))
  (Development|PrintString "NumberProvide is NULL" (!= (Utilities|IsValid _returnvalue) true) (!= (Utilities|IsValid _returnvalue) true))
  (bind _output_get (Variables|Default|SetNumberProvider _returnvalue))
  (Default|SetupWeightedNumbers _output_get)
  ;[1 1 1] Setup Number Converter
  (bind _returnvalue_2 (Game|ConstructObjectfromClass "/Game/Project/Elian/HelperSystems/NumbersToTextConverter.NumbersToTextConverter_C"))
  (Development|PrintString "NumbersConverter NOT Valid" (!= (Utilities|IsValid _returnvalue_2) true))
  (Variables|Default|SetNumberConverter _returnvalue_2)
  ;[1 1 1] GameManager to Upgrades
  (Default|AddGameManagertoAllUpgrades (Variables|Default|GetUpgradeManager))
  ;[1 1 1] UI
  (CallFunction|InitSettingsUI)
  (CallFunction|InitShop)
  (CallFunction|InitHUD)
  (Variables|/Script/Engine.PlayerController|SetbShowMouseCursor (Game|GetPlayerController 0) true)
  (Default|ResetMagazineTotalValue (Variables|Default|GetHUD_Widget))
  (CallFunction|InitMainMenu)
  (CallFunction|ShowMainMenu)
  (Utilities|FlowControl|Delay 0.2)
  (bind _returnvalue_3 (Actor|GetActorOfClass "/Game/Project/Mete/Camera/Blueprints/BP_Camera.BP_Camera_C"))
  (Default|MoveCameratoEnemy _returnvalue_3))

(event EventTick
  (params (DeltaSeconds :type Float%20%28single-precision%29))
  ;[1 1 1] Event Tick Countdown
  (if (Variables|Default|GetbRunTimer)
    (bind _output_get (Variables|Default|SetCurrentTimer (+ (Utilities|Time|GetWorldDeltaSeconds) (Variables|Default|GetCurrentTimer))))
    (if (>= _output_get 1.0)
      (Variables|Default|SetCurrentTimer 0.0)
      (bind _output_get_2 (Variables|Default|SetCurrentCountdownValue (- (Variables|Default|GetCurrentCountdownValue) 1)))
      (if (> _output_get_2 -1)
        (Default|UpdateTimer (Variables|Default|GetHUD_Widget) _output_get_2)
        (else
          (Variables|Default|SetbRunTimer false)
          (CallFunction|EnterGamemode2))))))

(fn ConstructionScript)

(fn ShootNextNumber
  (return (Utilities|Array|Get(acopy) (Variables|Default|GetMagazine))))

(fn GetNextNumber
  (return (Utilities|Array|Get(acopy) (Variables|Default|GetMagazine))))