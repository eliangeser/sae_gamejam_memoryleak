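; Upgrade Blueprint that doubles even numbers when they are collected.
; OnCollectEffect runs the parent effect first, tests its returned reference number for evenness, and outputs the parent's output number times two if even.
; CheckInt32Overflow flags values near or above half the int32 maximum, but both branches are empty, so doubling happens regardless.
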(fn OnCollectEffect
  (params (CollectedNumberRef :type Integer) (InputNumber :type Integer%20%28by%20ref%29))
  (bind (_outputnumberref _outputnumber) (|CallParentFunction CollectedNumberRef InputNumber))
  (Variables|Default|SetOutput%20Number _outputnumber)
  ;[1 1 1] Is Even Number ?
  (if (== (Math|Integer|%(Integer) _outputnumberref 2) 0)
    (bind _hasoverflown (CallFunction|CheckInt32Overflow _outputnumber))
    (if _hasoverflown
      _
      (else
        _))
    (Variables|Default|SetOutput%20Number (* _outputnumber 2)))
  (return _outputnumber (Variables|Default|GetOutput%20Number)))

(fn CheckInt32Overflow
  (params (InputNumber :type Integer))
  (return (>= InputNumber 1073741822)))