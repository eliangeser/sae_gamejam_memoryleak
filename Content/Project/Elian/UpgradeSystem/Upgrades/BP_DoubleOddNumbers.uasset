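; Upgrade Blueprint that doubles the output number on collection when the parent effect's reference number is odd.
; OnCollectEffect runs the parent effect first, then passes even cases through unchanged or multiplies the output by two.
; Before doubling, CheckInt32Overflow tests against roughly half the int32 limit; on a hit, it still doubles but sets the player overflow flag on GameManager.
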(fn OnCollectEffect
  (params (CollectedNumberRef :type Integer) (InputNumber :type Integer%20%28by%20ref%29))
  (bind (_outputnumberref _outputnumber) (|CallParentFunction CollectedNumberRef InputNumber))
  (Variables|Default|SetOutput%20Number _outputnumber)
  ;[1 1 1] Is Even Number ?
  (if (== (Math|Integer|%(Integer) _outputnumberref 2) 0)
    _
    (else
      ;[1 1 1] Check for overflow
      (bind _hasoverflown (CallFunction|CheckInt32Overflow _outputnumber))
      ;[1 1 1] Upgrade Regardless
      (Variables|Default|SetOutput%20Number (* _outputnumber 2))
      (if _hasoverflown
        ;[1 1 1] SettingPlayer Overflow Bool
        (if (Utilities|IsValid (Variables|Default|GetGameManager))
          (Default|SetPlayerOverflowBool (Variables|Default|GetGameManager) true)
          (else
            (Development|PrintString 0 "ERROR: GameManagerVariable NOT assigned in Upgrade")))
        (return _outputnumberref (Variables|Default|GetOutput%20Number))
        (else
          _))))
  (return _outputnumberref (Variables|Default|GetOutput%20Number)))

(fn CheckInt32Overflow
  (params (InputNumber :type Integer))
  (return (>= InputNumber 1073741822)))