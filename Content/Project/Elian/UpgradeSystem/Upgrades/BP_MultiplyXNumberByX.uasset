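; Upgrade Blueprint that multiplies a collected number by MultiplyAmount when its reference matches MulitplyNumber.
; OnCollectEffect runs the parent effect first, then applies the multiplier to that output and passes non-matching numbers through unchanged.
; CheckInt32Overflows compares against hardcoded int32 limits for 2x, 5x, 10x and 15x only.
; A detected overflow sets the GameManager's player overflow flag, but the multiplication still happens.
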(fn OnCollectEffect
  (params (CollectedNumberRef :type Integer) (InputNumber :type Integer%20%28by%20ref%29))
  (bind (_outputnumberref _outputnumber) (|CallParentFunction CollectedNumberRef InputNumber))
  (if (== _outputnumberref (Variables|Default|GetMulitplyNumber))
    (bind _hasoverflown (CallFunction|CheckInt32Overflows _outputnumber))
    (if _hasoverflown
      ;[1 1 1] SetPlayerOverlfow Bool to true
      (if (Utilities|IsValid (Variables|Default|GetGameManager))
        (Default|SetPlayerOverflowBool (Variables|Default|GetGameManager) true)
        (else
          (Development|PrintString 0 "ERROR: GameManagerVariable NOT assigned in Upgrade")
          (return _outputnumberref (* _outputnumber (Variables|Default|GetMultiplyAmount))))))
    (return _outputnumberref (* _outputnumber (Variables|Default|GetMultiplyAmount)))
    (else
      (return _outputnumberref _outputnumber))))

(fn CheckInt32Overflows
  (params (InputNumber :type Integer))
  (return (Math|Boolean|ORBoolean (and (>= InputNumber 1073741822) (== (Variables|Default|GetMultiplyAmount) 2)) (and (>= InputNumber 429496728) (== (Variables|Default|GetMultiplyAmount) 5)) (and (>= InputNumber 214748363) (== (Variables|Default|GetMultiplyAmount) 10)) (and (>= InputNumber 143165575) (== (Variables|Default|GetMultiplyAmount) 15)))))