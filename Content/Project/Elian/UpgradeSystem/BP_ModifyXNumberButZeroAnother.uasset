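; An upgrade that remaps collected numbers: one chosen number becomes a new value while another becomes worth zero.
; Setup stores the three numbers and builds the upgrade's descriptive text from them.
; OnCollectEffect runs the parent effect, then compares the returned number reference to both targets, outputting the new value, zero, or the parent's result unchanged.
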(event Custom|Setup
  (params (NumberToModify :type Integer) (New%20Value :type Integer) (NumberToZero :type Integer))
  (Variables|Default|SetNumberToModify NumberToModify)
  (Variables|Default|SetNewValue New%20Value)
  (Variables|Default|SetNumberToZero NumberToZero)
  (Variables|Default|SetUpgradeText (Utilities|String|BuildString(Integer) "" (Utilities|String|BuildString(Integer) "" (Utilities|String|BuildString(Integer) "" "Every " NumberToModify " becomes a ") New%20Value " but ") NumberToZero "s are worth 0")))

(fn OnCollectEffect
  (params (CollectedNumberRef :type Integer) (InputNumber :type Integer%20%28by%20ref%29))
  (bind (_outputnumberref _outputnumber) (|CallParentFunction CollectedNumberRef InputNumber))
  (if (== _outputnumberref (Variables|Default|GetNumberToModify))
    (return _outputnumberref (Variables|Default|GetNewValue))
    (elif (== _outputnumberref (Variables|Default|GetNumberToZero))
      (return _outputnumberref 0)
      (else
        (return _outputnumberref _outputnumber)))))