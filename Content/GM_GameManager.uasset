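; Game manager that drives the main menu, HUD, shop, round countdown and ammo magazine.
; BeginPlay creates the HUD and opens the main menu with the cursor; showing the HUD starts a self-recursive one-second countdown that updates the timer, then calls a still-empty EnterGamemode2.
; The magazine is a front-first stack of numeric values: removal drains the top entry, recursively carries any excess into the next and refreshes the HUD.
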(event Custom|StartCountDown
  ;[1 1 1] CountDown
  (if (> (Variables|Default|GetCurrentCountdownValue) 0.0)
    (Utilities|FlowControl|Delay 1.0)
    (bind _output_get (Variables|Default|SetCurrentCountdownValue (+ (Variables|Default|GetCurrentCountdownValue) -1.0)))
    (Default|UpdateTimer (Variables|Default|GetHUD_Widget) (Math|Float|Truncate (Math|Conversions|ToFloat(Integer) _output_get)))
    (CallFunction|StartCountDown)
    (else
      (CallFunction|EnterGamemode2))))

(event Custom|ResetCountdown
  ;[1 1 1] CountDown
  (Variables|Default|SetCurrentCountdownValue (Variables|Default|GetMaxCountdownValue))
  (CallFunction|StartCountDown))

(event Custom|DebugMagazineLength
  ;[1 1 1] Magazine
  (Development|PrintString (Utilities|String|ToString(Integer) (Utilities|Array|Length (Variables|Default|GetMagazine)))))

(event Custom|RemoveAmmoAmount
  (params (AmountToRemove :type Integer))
  (bind _magazine (Variables|Default|GetMagazine))
  (bind _output (Utilities|Array|Get(acopy) _magazine))
  ;[1 1 1] Magazine
  (if (> AmountToRemove 0)
    (bind _output_get (Variables|Default|SetAmmoLossCount AmountToRemove))
    (if (> _output_get _output)
      (bind _output_get_2 (Variables|Default|SetAmmoLossCount (- (Variables|Default|GetAmmoLossCount) (Utilities|Array|Get(acopy) (Variables|Default|GetMagazine)))))
      (CallFunction|RemoveTopAmmo)
      (if (> (Utilities|Array|Length (Variables|Default|GetMagazine)) 0)
        (CallFunction|RemoveAmmoAmount _output_get_2))
      (elif (> (- _output (Variables|Default|GetAmmoLossCount)) 0)
        (Utilities|Array|SetArrayElem (Variables|Default|GetMagazine) 0 (- _output (Variables|Default|GetAmmoLossCount)))
        (CallFunction|UpdateMagazineUI)
        (else
          (CallFunction|RemoveTopAmmo))))))

(event Custom|RemoveTopAmmo
  ;[1 1 1] Magazine
  (Utilities|Array|RemoveIndex (Variables|Default|GetMagazine))
  (CallFunction|UpdateMagazineUI))

(event Custom|UpdateMagazineUI
  ;[1 1 1] Magazine
  (Default|UpdateMagazineUI (Variables|Default|GetHUD_Widget)))

(event Custom|EnterGamemode2)

(event Custom|ShowMainMenu
  (bind _returnvalue (UserInterface|CreateWidget "/Game/GUI/WB_MainMenu.WB_MainMenu_C"))
  (UserInterface|Viewport|AddtoViewport _returnvalue 0))

(event Custom|InitHUD
  (bind _returnvalue (UserInterface|CreateWidget "/Game/GUI/WB_HUD.WB_HUD_C"))
  (Variables|Default|SetHUD_Widget _returnvalue)
  (Variables|Default|SetCurrentCountdownValue (Variables|Default|GetMaxCountdownValue)))

(event Custom|ShowShop
  (bind _returnvalue (UserInterface|CreateWidget "/Game/GUI/WB_Shop.WB_Shop_C"))
  (UserInterface|Viewport|AddtoViewport _returnvalue 0)
  (Variables|/Script/Engine.PlayerController|SetbShowMouseCursor (Game|GetPlayerController 0) true))

(event Custom|HideHUD
  (Widget|RemovefromParent (Variables|Default|GetHUD_Widget))
  (Variables|Default|SetCurrentCountdownValue (Variables|Default|GetMaxCountdownValue)))

(event Custom|ShowHUD
  (UserInterface|Viewport|AddtoViewport (Variables|Default|GetHUD_Widget) 0)
  (CallFunction|StartCountDown))

(event Custom|AddAmmo
  (params (NewNumber :type Integer))
  ;[1 1 1] Magazine
  (CallFunction|DebugMagazineLength)
  (Utilities|Array|Insert (Variables|Default|GetMagazine) NewNumber)
  (CallFunction|DebugMagazineLength)
  (Default|UpdateMagazineUI (Variables|Default|GetHUD_Widget)))

(event EventBeginPlay
  (CallFunction|InitHUD)
  (CallFunction|ShowMainMenu)
  (Variables|/Script/Engine.PlayerController|SetbShowMouseCursor (Game|GetPlayerController 0) true)
  (Default|ResetMagazineUI (Variables|Default|GetHUD_Widget)))

(event EventTick
  (params (DeltaSeconds :type Float%20%28single-precision%29)))

(fn ConstructionScript)